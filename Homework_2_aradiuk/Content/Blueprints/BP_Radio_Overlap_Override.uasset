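; Radio actor whose audio becomes audible or silent based on overlaps with its box collision.
; BeginPlay binds the box's begin and end overlap events and starts the audio unpaused at zero volume.
; Both overlaps pass the actor and a pause flag to TurnSound, which is defined outside this file.
; SwitchRadio maps a pause flag to zero or full volume, muting without pausing playback.
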(event `self.ReceiveBeginPlay`
  (bind _boxcollision (`self.BoxCollision`))
  (bind _audio (`self.Audio`))
  (add `PrimitiveComponent.OnComponentBeginOverlap` _boxcollision (delegate `OnComponentBeginOverlap_Event_0`))
  (add `PrimitiveComponent.OnComponentEndOverlap` _boxcollision (delegate `OnComponentEndOverlap_Event_0`))
  (`AudioComponent.SetVolumeMultiplier` _audio 0.0)
  (`AudioComponent.SetPaused` _audio false))

(event `OnComponentBeginOverlap_Event_0`
  (params (OverlappedComponent :type "PrimitiveComponent Object Reference") (OtherActor :type "Actor Object Reference") (OtherComp :type "PrimitiveComponent Object Reference") (OtherBodyIndex :type Integer) (bFromSweep :type Boolean) (SweepResult :type "HitResult Structure (by ref)"))
  (`self.TurnSound` OtherActor))

(event `OnComponentEndOverlap_Event_0`
  (params (OverlappedComponent :type "PrimitiveComponent Object Reference") (OtherActor :type "Actor Object Reference") (OtherComp :type "PrimitiveComponent Object Reference") (OtherBodyIndex :type Integer))
  (`self.TurnSound` OtherActor true))

(event `self.SwitchRadio`
  (params (isPaused :type Boolean))
  (bind _audio (`self.Audio`))
  (if isPaused
    (`AudioComponent.SetVolumeMultiplier` _audio 0.0)
    (else
      (`AudioComponent.SetVolumeMultiplier` _audio 1.0))))

(fn `UserConstructionScript`)